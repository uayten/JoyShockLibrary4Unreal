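; Game mode that spawns local players for controllers reported by the JoyShock subsystem.
; On BeginPlay it binds connect and disconnect events.
; Each connect event loops over all connected controllers, creating a player for any with a nonzero player index and mapping device ID to player controller.
; The disconnect handler looks up the mapped controller and compares it to player 0, but takes no action.
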(event Custom|OnControllerConnected_Event
  (params (DeviceId :type Integer))
  (bind _returnvalue (Class|JoyShockLibrary|JSL4UGetConnectedControllers))
  (for _array_element _returnvalue
    (Variables|Default|SetCurrent%20Device%20ID (.deviceid _array_element))
    (if (not (== (.playerindex _array_element) 0))
      (bind _returnvalue_2 (Class|GameplayStatics|CreatePlayer (Variables|Default|GetCurrent%20Device%20ID)))
      (Utilities|Map|Add (Variables|Default|GetPlayerControllerByDeviceID) (Variables|Default|GetCurrent%20Device%20ID) _returnvalue_2))))

(event Custom|OnControllerDisconnected_Event
  (params (DeviceId :type Integer) (bTimedOut :type Boolean))
  (bind _playercontrollerbydeviceid (Variables|Default|GetPlayerControllerByDeviceID))
  (bind (_value _returnvalue) (Utilities|Map|Find _playercontrollerbydeviceid DeviceId))
  (if _returnvalue
    (if (== _value (Game|GetPlayerController 0))
      _)))

(event EventBeginPlay
  (bind _returnvalue (Subsystems|GetJoyShockSubsystem))
  (EventDispatchers|AssignOnControllerConnected _returnvalue (delegate Custom|OnControllerConnected_Event))
  (EventDispatchers|BindEventtoOnControllerDisconnected _returnvalue (delegate Custom|OnControllerDisconnected_Event)))

(fn ConstructionScript)