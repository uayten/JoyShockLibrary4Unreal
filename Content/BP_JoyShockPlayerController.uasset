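; BP_JoyShockPlayerController is a test player controller that checks gamepad button input with the JoyShock (JSL4U) plugin.
; Each key event prints the button's name, covering standard gamepad buttons plus SL/SR, touchpad/capture, Home/PS and Pro Controller 2 grip and chat buttons.
; The left trigger also queries connected controllers, and both it and the left shoulder set device 0's rumble to zero.
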(event Input|GamepadEvents|GamepadDPadDown
  (params (Key :type Key%20Structure :default "None"))
  ;[0.15 0.15 0.15 0.5] D-Buttons
  (:Pressed
    (Development|PrintString "D-pad Down")))

(event Input|GamepadEvents|GamepadDPadRight
  (params (Key :type Key%20Structure :default "None"))
  ;[0.15 0.15 0.15 0.5] D-Buttons
  (:Pressed
    (Development|PrintString "D-pad Right")))

(event Input|GamepadEvents|GamepadLeftThumbstick
  (params (Key :type Key%20Structure :default "None"))
  ;[0.15 0.15 0.15 0.5] Direcionais
  (:Pressed
    (Development|PrintString "Left Thumbstick Button")))

(event Input|GamepadEvents|GamepadRightThumbstick
  (params (Key :type Key%20Structure :default "None"))
  ;[0.15 0.15 0.15 0.5] Direcionais
  (:Pressed
    (Development|PrintString "Right Thumbstick Button")))

(event Input|GamepadEvents|GamepadLeftShoulder
  (params (Key :type Key%20Structure :default "None"))
  ;[0.15 0.15 0.15 0.5] Gatilhos
  (:Pressed
    (Development|PrintString "L")
    (Class|JoyShockLibrary|JslSetRumble)))

(event Input|GamepadEvents|GamepadRightShoulder
  (params (Key :type Key%20Structure :default "None"))
  ;[0.15 0.15 0.15 0.5] Gatilhos
  (:Pressed
    (Development|PrintString "R")))

(event Input|GamepadEvents|GamepadLeftTrigger
  (params (Key :type Key%20Structure :default "None"))
  ;[0.15 0.15 0.15 0.5] Gatilhos
  (:Pressed
    (Development|PrintString "ZL")
    (Class|JoyShockLibrary|JSL4UGetConnectedControllers)
    (Class|JoyShockLibrary|JslSetRumble)))

(event Input|GamepadEvents|GamepadRightTrigger
  (params (Key :type Key%20Structure :default "None"))
  ;[0.15 0.15 0.15 0.5] Gatilhos
  (:Pressed
    (Development|PrintString "ZR")))

(event Input|KeyboardEvents|PS
  (params (Key :type Key%20Structure :default "None"))
  ;[0.15 0.15 0.15 0.5] Home
  (:Pressed
    (Development|PrintString "Home / PS")))

(event Input|KeyboardEvents|SwitchC
  (params (Key :type Key%20Structure :default "None"))
  ;[0.15 0.15 0.15 0.5] Voice
  (:Pressed
    (Development|PrintString "Game Chat (Pro Controller 2)")))

(event Input|GamepadEvents|GamepadDPadUp
  (params (Key :type Key%20Structure :default "None"))
  ;[0.15 0.15 0.15 0.5] D-Buttons
  (:Pressed
    (Development|PrintString "D-pad Up")))

(event Input|KeyboardEvents|GripLeft
  (params (Key :type Key%20Structure :default "None"))
  ;[0.15 0.15 0.15 0.5] Macro Right
  (:Pressed
    (Development|PrintString "Grip Left (Pro Controller 2)")))

(event Input|KeyboardEvents|GripRight
  (params (Key :type Key%20Structure :default "None"))
  ;[0.15 0.15 0.15 0.5] Macro Left
  (:Pressed
    (Development|PrintString "Grip Right (Pro Controller 2)")))

(event Input|TouchEvents|TouchPadClick
  (params (Key :type Key%20Structure :default "None"))
  ;[0.15 0.15 0.15 0.5] Print
  (:Pressed
    (Development|PrintString "Capture / Touch Pad Click")))

(event Input|KeyboardEvents|SideLeft
  (params (Key :type Key%20Structure :default "None"))
  ;[0.15 0.15 0.15 0.5] +-
  (:Pressed
    (Development|PrintString "SL")))

(event Input|KeyboardEvents|SideRight
  (params (Key :type Key%20Structure :default "None"))
  ;[0.15 0.15 0.15 0.5] +-
  (:Pressed
    (Development|PrintString "SR")))

(event Input|GamepadEvents|GamepadDPadLeft
  (params (Key :type Key%20Structure :default "None"))
  ;[0.15 0.15 0.15 0.5] D-Buttons
  (:Pressed
    (Development|PrintString "D-pad Left")))

(event Input|GamepadEvents|GamepadFaceButtonBottom
  (params (Key :type Key%20Structure :default "None"))
  ;[0.15 0.15 0.15 0.5] ABXY
  (:Pressed
    (Development|PrintString "Face Button Bottom")))

(event Input|GamepadEvents|GamepadFaceButtonTop
  (params (Key :type Key%20Structure :default "None"))
  ;[0.15 0.15 0.15 0.5] ABXY
  (:Pressed
    (Development|PrintString "Face Button Top")))

(event Input|GamepadEvents|GamepadFaceButtonLeft
  (params (Key :type Key%20Structure :default "None"))
  ;[0.15 0.15 0.15 0.5] ABXY
  (:Pressed
    (Development|PrintString "Face Button Left")))

(event Input|GamepadEvents|GamepadFaceButtonRight
  (params (Key :type Key%20Structure :default "None"))
  ;[0.15 0.15 0.15 0.5] ABXY
  (:Pressed
    (Development|PrintString "Face Button Right")))

(event Input|GamepadEvents|GamepadSpecialLeft
  (params (Key :type Key%20Structure :default "None"))
  ;[0.15 0.15 0.15 0.5] +-
  (:Pressed
    (Development|PrintString "-/Special Left")))

(event Input|GamepadEvents|GamepadSpecialRight
  (params (Key :type Key%20Structure :default "None"))
  ;[0.15 0.15 0.15 0.5] +-
  (:Pressed
    (Development|PrintString "+/Special Right")))

(fn ConstructionScript)