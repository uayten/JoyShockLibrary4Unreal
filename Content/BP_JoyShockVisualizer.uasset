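; Actor that visualizes a JoyShock motion controller, using a Joy-Con mesh or the DualSense mesh for all other types.
; Tick optionally copies the device's orientation to the actor (RotationMode) and moves it in Y/Z by flushed accumulated gyro within clamped bounds (AimMode).
; Custom events toggle these modes and tick, and exercise the JoyShock API for gyro space, calibration, connecting and connection checks.
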(event Custom|StillConnected
  (bind _returnvalue (Class|JoyShockLibrary|JslStillConnected (Variables|Default|GetDeviceID)))
  (Development|PrintString (Utilities|String|ToString(Boolean) _returnvalue) true false))

(event Custom|ConnectDevices
  (bind _returnvalue (Class|JoyShockLibrary|JslConnectDevices))
  (Development|PrintString (Utilities|String|ToString(Integer) _returnvalue) true false)
  (Actor|Tick|SetActorTickEnabled true))

(event Custom|ToggleRotationMode
  (Variables|Default|SetbRotationMode (not (Variables|Default|GetbRotationMode))))

(event Custom|ToggleAimMode
  (Variables|Default|SetbAimMode (not (Variables|Default|GetbAimMode))))

(event Custom|ToggleTick
  (Actor|Tick|SetActorTickEnabled (not (Class|Actor|IsActorTickEnabled))))

(event Custom|SetAutomaticCalibration
  (bind _deviceid (Variables|Default|GetDeviceID))
  (bind _returnvalue (Class|JoyShockLibrary|JslGetAutoCalibrationStatus _deviceid))
  (bind _returnvalue_2 (not (.autocalibrationenabled _returnvalue)))
  (Class|JoyShockLibrary|JslSetAutomaticCalibration (Variables|Default|GetDeviceID) _returnvalue_2)
  (Development|PrintString (Utilities|String|ToString(Boolean) _returnvalue_2) true false))

(event Custom|StartContinuousCalibration
  (Class|JoyShockLibrary|JslStartContinuousCalibration (Variables|Default|GetDeviceID)))

(event Custom|PauseContinuousCalibration
  (Class|JoyShockLibrary|JslPauseContinuousCalibration (Variables|Default|GetDeviceID)))

(event Custom|LocalSpace
  (Class|JoyShockLibrary|JslSetGyroSpace (Variables|Default|GetDeviceID)))

(event Custom|PlayerSpace
  (Class|JoyShockLibrary|JslSetGyroSpace (Variables|Default|GetDeviceID) 2))

(event Custom|WorldSpace
  (Class|JoyShockLibrary|JslSetGyroSpace (Variables|Default|GetDeviceID) 1))

(event EventBeginPlay
  (bind _current_controller_info (Variables|Default|GetCurrent%20Controller%20Info))
  (Variables|Default|SetDeviceID (.deviceid _current_controller_info))
  (CallFunction|SetControllerStaticMesh (Variables|Default|GetController) (.controllertype _current_controller_info)))

(event EventTick
  (params (DeltaSeconds :type Float%20%28single-precision%29))
  (bind _returnvalue (Transformation|GetActorLocation))
  (Utilities|FlowControl|Sequence
    (:then_0
      (if (Variables|Default|GetbRotationMode)
        (Transformation|SetActorRotation (Class|KismetMathLibrary|QuatRotator (.orientation (Class|JoyShockLibrary|JSL4UGetMotionState (Variables|Default|GetDeviceID)))))))
    (:then_1
      (if (Variables|Default|GetbAimMode)
        (bind _returnvalue_2 (Class|JoyShockLibrary|JSL4UGetandFlushAccumulatedGyro (Variables|Default|GetDeviceID)))
        (Development|PrintText (Utilities|Text|ToText(String) _returnvalue_2) true false "(R=0.000000,G=0.660000,B=1.000000,A=1.000000)" 0.0)
        (Transformation|AddActorWorldOffset (Math|Vector|MakeVector 0.0 (.Z (Math|Vector|BreakVector _returnvalue_2)) (.Y (Math|Vector|BreakVector _returnvalue_2))))
        (Transformation|SetActorLocation (Math|Vector|MakeVector (.x _returnvalue) (Math|Float|Clamp(Float) (.y _returnvalue) -5e+02 5e+02) (Math|Float|Clamp(Float) (.z _returnvalue) -1.5e+02 4e+02)) false false)))))

(fn ConstructionScript)

(fn SetControllerStaticMesh
  (params (Static%20Mesh%20Component :type Static%20Mesh%20Component%20Object%20Reference) (Controller%20Type :type EJSL4UControllerType%20Enum :default "Undefined"))
  (switch Utilities|FlowControl|Switch|SwitchonEJSL4UControllerType Controller%20Type
    (:Undefined
      (Components|StaticMesh|SetStaticMesh Static%20Mesh%20Component "/JoyShockLibrary4Unreal/Meshes/DualSense/SM_Dual_Sense.SM_Dual_Sense" :!label _label))
    (:JoyConLeft
      (Components|StaticMesh|SetStaticMesh Static%20Mesh%20Component "/JoyShockLibrary4Unreal/Meshes/Nintendo/Joy-Con(L)/Joy-Con_L.Joy-Con_L"))
    (:JoyConRight
      (Components|StaticMesh|SetStaticMesh Static%20Mesh%20Component "/JoyShockLibrary4Unreal/Meshes/Nintendo/Joy-Con(R)/SM_Joy-Con_R.SM_Joy-Con_R"))
    (:ProController
      (goto _label))
    (:DualShock4
      (goto _label))
    (:DualSense
      (goto _label))
    (:ProController2
      (goto _label))))