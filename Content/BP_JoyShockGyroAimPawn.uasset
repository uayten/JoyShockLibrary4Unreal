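; Pawn for a JoyShock gyro aim demo that turns the view with controller gyro and both sticks.
; On possession it adds the input mapping and creates a settings overlay.
; Gyro and stick input, scaled by delta time, feed a shared Turn that clamps pitch on the control rotation.
; D-pad tunes gyro sensitivity, stick clicks toggle inversion with controller-specific overlay hints, and the right face button spawns a mark at a camera trace hit.
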(event Custom|Stick%20Turn
  (params (Value :type Vector%202D%20Structure))
  (bind (_x _y) (Math|Vector2D|BreakVector2D Value))
  (bind _returnvalue (Utilities|Time|GetWorldDeltaSeconds))
  (bind _stick_speed (Variables|Default|GetStick%20Speed))
  (bind _returnvalue_2 (* _returnvalue _stick_speed))
  (CallFunction|Turn (* _y (* _returnvalue_2 (Math|Float|SelectFloat -1.0 1.0 (Variables|Default|GetInvert%20Stick%20X)))) (* _x (* _returnvalue_2 (Math|Float|SelectFloat 1.0 -1.0 (Variables|Default|GetInvert%20Stick%20Y))))))

(event Custom|Turn
  (params (Yaw :type Float%20%28double-precision%29) (Pitch :type Float%20%28double-precision%29))
  (bind _returnvalue (Pawn|GetControlRotation :!class /Script/Engine.Pawn))
  (bind (_roll _pitch _yaw) (Math|Rotator|BreakRotator _returnvalue))
  (Pawn|SetControlRotation (Pawn|GetController) (Math|Rotator|MakeRotator 0.0 (Math|Float|ClampAngle (+ _pitch Pitch) -89.0 89.0) (+ _yaw Yaw))))

(event Custom|Change%20Gyro%20Sensitivity
  (params (Horizontal%20Step :type Float%20%28double-precision%29) (Vertical%20Step :type Float%20%28double-precision%29))
  (CallFunction|ApplyGyroSensitivity (+ (Variables|Default|GetGyro%20Sensitivity%20Horizontal) Horizontal%20Step) (+ (Variables|Default|GetGyro%20Sensitivity%20Vertical) Vertical%20Step)))

(event Custom|Apply%20Gyro%20Sensitivity
  (params (Horizontal :type Float%20%28double-precision%29) (Vertical :type Float%20%28double-precision%29))
  (Variables|Default|SetGyro%20Sensitivity%20Horizontal (Math|Float|Clamp(Float) Horizontal 0.1 5.0))
  (Variables|Default|SetGyro%20Sensitivity%20Vertical (Math|Float|Clamp(Float) Vertical 0.1 5.0))
  (CallFunction|ShowAimSettings))

(event Custom|Toggle%20Invert%20Stick%20X
  (Variables|Default|SetInvert%20Stick%20X (not (Variables|Default|GetInvert%20Stick%20X)))
  (CallFunction|ShowAimSettings))

(event Custom|Toggle%20Invert%20Stick%20Y
  (Variables|Default|SetInvert%20Stick%20Y (not (Variables|Default|GetInvert%20Stick%20Y)))
  (CallFunction|ShowAimSettings))

(event Custom|Show%20Aim%20Settings
  (bind _overlay (Variables|Default|GetOverlay))
  (bind _gyro_sensitivity_horizontal (Variables|Default|GetGyro%20Sensitivity%20Horizontal))
  (bind _gyro_sensitivity_vertical (Variables|Default|GetGyro%20Sensitivity%20Vertical))
  (bind _selected_id (Variables|/JoyShockLibrary4Unreal/UI/WBP_JoyShockGyroAimOverlay.WBP_JoyShockGyroAimOverlay_C|GetSelected%20Id _overlay))
  (bind _returnvalue (Class|JoyShockLibrary|JSL4UGetControllerInfo _selected_id))
  (bind (_bisjoyshockcontroller _connectionid _inputdeviceid _platformuserid _hardwaredeviceidentifier _controllertype _playerindex _joinedtoconnectionid) (Utilities|Struct|BreakJSL4UControllerInfo _returnvalue))
  (bind _returnvalue_2 (== _joinedtoconnectionid 0))
  (bind _returnvalue_3 (Utilities|Enum|Equal(Enum) _controllertype "JoyConRight"))
  (bind _returnvalue_4 (Utilities|Enum|Equal(Enum) _controllertype "JoyCon2Right"))
  (bind _returnvalue_5 (Utilities|Enum|Equal(Enum) _controllertype "DualShock4"))
  (bind _returnvalue_6 (Utilities|Enum|Equal(Enum) _controllertype "DualSense"))
  (bind _returnvalue_7 (Utilities|Enum|Equal(Enum) _controllertype "JoyConLeft"))
  (bind _returnvalue_8 (Utilities|Enum|Equal(Enum) _controllertype "JoyCon2Left"))
  (bind _returnvalue_9 (or _returnvalue_5 _returnvalue_6))
  (bind _returnvalue_10 (Math|Boolean|ORBoolean _returnvalue_7 _returnvalue_8 _returnvalue_3 _returnvalue_4))
  (bind _returnvalue_11 (and _returnvalue_10 _returnvalue_2))
  (if (Utilities|IsValid _overlay)
    (Rendering|Components|TextRender|SetText (Variables|/JoyShockLibrary4Unreal/UI/WBP_JoyShockGyroAimOverlay.WBP_JoyShockGyroAimOverlay_C|GetGyroHorizontalText _overlay) (Utilities|Text|ToText(String) (Utilities|String|Append "Gyro horizontal (D-pad left/right): " (Utilities|String|ToString(Text) (Utilities|Text|ToText(Float) _gyro_sensitivity_horizontal "HalfToEven" false true 1 324 1 1)))))
    (Class|Slider|SetValue (Variables|/JoyShockLibrary4Unreal/UI/WBP_JoyShockGyroAimOverlay.WBP_JoyShockGyroAimOverlay_C|GetGyroHorizontalSlider _overlay) _gyro_sensitivity_horizontal)
    (Rendering|Components|TextRender|SetText (Variables|/JoyShockLibrary4Unreal/UI/WBP_JoyShockGyroAimOverlay.WBP_JoyShockGyroAimOverlay_C|GetGyroVerticalText _overlay) (Utilities|Text|ToText(String) (Utilities|String|Append "Gyro vertical (D-pad up/down): " (Utilities|String|ToString(Text) (Utilities|Text|ToText(Float) _gyro_sensitivity_vertical "HalfToEven" false true 1 324 1 1)))))
    (Class|Slider|SetValue (Variables|/JoyShockLibrary4Unreal/UI/WBP_JoyShockGyroAimOverlay.WBP_JoyShockGyroAimOverlay_C|GetGyroVerticalSlider _overlay) _gyro_sensitivity_vertical)
    (Rendering|Components|TextRender|SetText (Variables|/JoyShockLibrary4Unreal/UI/WBP_JoyShockGyroAimOverlay.WBP_JoyShockGyroAimOverlay_C|GetInvertXText _overlay) (Utilities|Text|ToText(String) (Utilities|String|Append "Invert stick X: " (Utilities|String|SelectString "on" "off" (Variables|Default|GetInvert%20Stick%20X)) "   (" (Utilities|String|SelectString "press L3" (Utilities|String|SelectString "press the stick" "press the left stick" _returnvalue_11) _returnvalue_9) ")")))
    (Rendering|Components|TextRender|SetText (Variables|/JoyShockLibrary4Unreal/UI/WBP_JoyShockGyroAimOverlay.WBP_JoyShockGyroAimOverlay_C|GetInvertYText _overlay) (Utilities|Text|ToText(String) (Utilities|String|Append "Invert stick Y: " (Utilities|String|SelectString "on" "off" (Variables|Default|GetInvert%20Stick%20Y)) "   (" (Utilities|String|SelectString "press R3" (Utilities|String|SelectString "click here" "press the right stick" _returnvalue_11) _returnvalue_9) ")")))))

(event Input|EnhancedActionEvents|EnhancedInputActionJoyShock-GyroscopeRotation
  (params (ActionValue :type Vector :default "0, 0, 0") (ElapsedSeconds :type Float%20%28double-precision%29) (TriggeredSeconds :type Float%20%28double-precision%29) (InputAction :type Input%20Action%20Object%20Reference :default "/JoyShockLibrary4Unreal/EnhancedInput/JoyShock-GyroscopeRotation.JoyShock-GyroscopeRotation"))
  (bind _returnvalue (Utilities|Time|GetWorldDeltaSeconds))
  (bind (_x _y _z) (Math|Vector|BreakVector ActionValue))
  (CallFunction|Turn (* (* _z (Variables|Default|GetGyro%20Sensitivity%20Horizontal)) _returnvalue) (* (* _y (Variables|Default|GetGyro%20Sensitivity%20Vertical)) _returnvalue)))

(event Input|EnhancedActionEvents|EnhancedInputActionJoyShock-RightJoystick
  (params (ActionValue :type Vector%202D%20Structure) (ElapsedSeconds :type Float%20%28double-precision%29) (TriggeredSeconds :type Float%20%28double-precision%29) (InputAction :type Input%20Action%20Object%20Reference :default "/JoyShockLibrary4Unreal/EnhancedInput/JoyShock-RightJoystick.JoyShock-RightJoystick"))
  (CallFunction|StickTurn ActionValue))

(event Input|EnhancedActionEvents|EnhancedInputActionJoyShock-LeftJoystick
  (params (ActionValue :type Vector%202D%20Structure) (ElapsedSeconds :type Float%20%28double-precision%29) (TriggeredSeconds :type Float%20%28double-precision%29) (InputAction :type Input%20Action%20Object%20Reference :default "/JoyShockLibrary4Unreal/EnhancedInput/JoyShock-LeftJoystick.JoyShock-LeftJoystick"))
  (CallFunction|StickTurn (* ActionValue "(X=-1.000000,Y=1.000000)")))

(event Input|EnhancedActionEvents|EnhancedInputActionJoyShock-FaceButtonRight
  (params (ActionValue :type Boolean) (ElapsedSeconds :type Float%20%28double-precision%29) (TriggeredSeconds :type Float%20%28double-precision%29) (InputAction :type Input%20Action%20Object%20Reference :default "/JoyShockLibrary4Unreal/EnhancedInput/JoyShock-FaceButtonRight.JoyShock-FaceButtonRight"))
  (bind _camera (Variables|Default|GetCamera))
  (bind _returnvalue (Transformation|GetWorldLocation _camera))
  (:Started
    (bind (_outhit _returnvalue_2) (Collision|LineTraceByChannel _returnvalue (+ _returnvalue (* (Math|Vector|GetForwardVector _camera) 1e+04)) "TraceTypeQuery1" false 0 "None"))
    (if _returnvalue_2
      (Game|SpawnActorfromClass "/JoyShockLibrary4Unreal/BP_JoyShockGyroAimMark.BP_JoyShockGyroAimMark_C" (Math|Transform|MakeTransform (.Location (Collision|BreakHitResult _outhit)) "0, 0, 0" "1.000000,1.000000,1.000000") "Undefined" "MultiplyWithRoot" 0 0))))

(event Input|EnhancedActionEvents|EnhancedInputActionJoyShock-DPadUp
  (params (ActionValue :type Boolean) (ElapsedSeconds :type Float%20%28double-precision%29) (TriggeredSeconds :type Float%20%28double-precision%29) (InputAction :type Input%20Action%20Object%20Reference :default "/JoyShockLibrary4Unreal/EnhancedInput/JoyShock-DPadUp.JoyShock-DPadUp"))
  (CallFunction|ChangeGyroSensitivity 0.0 0.1))

(event Input|EnhancedActionEvents|EnhancedInputActionJoyShock-DPadDown
  (params (ActionValue :type Boolean) (ElapsedSeconds :type Float%20%28double-precision%29) (TriggeredSeconds :type Float%20%28double-precision%29) (InputAction :type Input%20Action%20Object%20Reference :default "/JoyShockLibrary4Unreal/EnhancedInput/JoyShock-DPadDown.JoyShock-DPadDown"))
  (CallFunction|ChangeGyroSensitivity 0.0 -0.1))

(event Input|EnhancedActionEvents|EnhancedInputActionJoyShock-DPadRight
  (params (ActionValue :type Boolean) (ElapsedSeconds :type Float%20%28double-precision%29) (TriggeredSeconds :type Float%20%28double-precision%29) (InputAction :type Input%20Action%20Object%20Reference :default "/JoyShockLibrary4Unreal/EnhancedInput/JoyShock-DPadRight.JoyShock-DPadRight"))
  (CallFunction|ChangeGyroSensitivity 0.1 0.0))

(event Input|EnhancedActionEvents|EnhancedInputActionJoyShock-DPadLeft
  (params (ActionValue :type Boolean) (ElapsedSeconds :type Float%20%28double-precision%29) (TriggeredSeconds :type Float%20%28double-precision%29) (InputAction :type Input%20Action%20Object%20Reference :default "/JoyShockLibrary4Unreal/EnhancedInput/JoyShock-DPadLeft.JoyShock-DPadLeft"))
  (CallFunction|ChangeGyroSensitivity -0.1 0.0))

(event Input|EnhancedActionEvents|EnhancedInputActionJoyShock-LeftThumb
  (params (ActionValue :type Boolean) (ElapsedSeconds :type Float%20%28double-precision%29) (TriggeredSeconds :type Float%20%28double-precision%29) (InputAction :type Input%20Action%20Object%20Reference :default "/JoyShockLibrary4Unreal/EnhancedInput/JoyShock-LeftThumb.JoyShock-LeftThumb"))
  (:Started
    (CallFunction|ToggleInvertStickX)))

(event Input|EnhancedActionEvents|EnhancedInputActionJoyShock-RightThumb
  (params (ActionValue :type Boolean) (ElapsedSeconds :type Float%20%28double-precision%29) (TriggeredSeconds :type Float%20%28double-precision%29) (InputAction :type Input%20Action%20Object%20Reference :default "/JoyShockLibrary4Unreal/EnhancedInput/JoyShock-RightThumb.JoyShock-RightThumb"))
  (:Started
    (CallFunction|ToggleInvertStickY)))

(event EventPossessed
  (params (NewController :type Controller%20Object%20Reference))
  (bind _returnvalue (Game|GetPlayerController 0))
  (bind _asplayer_controller (Utilities|Casting|CastToPlayerController NewController))
  (Input|AddMappingContext (PlayerController|LocalPlayerSubsystems|GetEnhancedInputLocalPlayerSubsystem _asplayer_controller) "/JoyShockLibrary4Unreal/EnhancedInput/JoyShockInputMappingContext.JoyShockInputMappingContext" 0 "(bIgnoreAllPressedKeysUntilRelease=True,bForceImmediately=False,bNotifyUserSettings=False)")
  (Game|Player|SetViewTargetwithBlend _returnvalue self 0.0 "VTBlend_Linear" 0.0 false)
  (if (Utilities|IsValid (Variables|Default|GetOverlay))
    (Utilities|FlowControl|DelayUntilNextTick)
    (Class|WidgetBlueprintLibrary|SetFocustoGameViewport)
    (else
      (bind _returnvalue_2 (UserInterface|CreateWidget "/JoyShockLibrary4Unreal/UI/WBP_JoyShockGyroAimOverlay.WBP_JoyShockGyroAimOverlay_C" _returnvalue))
      (UserInterface|Viewport|AddtoViewport _returnvalue_2 0)
      (Variables|Default|SetOverlay _returnvalue_2)
      (Variables|/Script/Engine.PlayerController|SetbShowMouseCursor _returnvalue true)
      (Input|SetInputModeGameandUI _returnvalue 0 "DoNotLock" false false)
      (CallFunction|ShowAimSettings))))

(fn ConstructionScript)