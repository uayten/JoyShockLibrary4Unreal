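; JoyShock demo initializer that sets up shared-screen local multiplayer for up to eight controllers.
; Async listeners handle connection, Joy-Con join/separate and blocked-function events, ensuring each controller has a local player, Enhanced Input mapping context and possessed character at a PlayerStart.
; Connections also spawn offset mirror actors, tracked by connection and device ID, and rebuild a diagnostics HUD from them.
; Disconnections destroy and untrack the mirrors.
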(event EventBeginPlay
  (Class|GameplayStatics|SetForceDisableSplitscreen true)
  (Class|JoyShockLibrary|JSL4USetMaxLocalPlayers 8)
  (bind _controller (|WaitforAnyControllerChanges)
    (:then
      (bind (_asynctaskproxy _leftjoycon _rightjoycon) (|WaitforJoyConPairingChanges)
        (:then
          (bind (_asynctaskproxy_2 _controller_2 _function) (|WaitforControllerFunctionBlocked)
            (:OnBlocked
              (Development|PrintString (Utilities|String|Append (Utilities|String|EnumtoString (.ControllerType (Utilities|Struct|BreakJSL4UControllerInfo _controller_2))) " had the " (Utilities|String|EnumtoString _function) " function blocked") true true "(R=0.000000,G=0.660000,B=1.000000,A=1.000000)" 5.0))))
        (:OnJoined
          (CallFunction|EnsureCharacterforController _leftjoycon))
        (:OnSeparated
          (CallFunction|EnsureCharacterforController _rightjoycon))))
    (:OnConnected
      (CallFunction|EnsureCharacterforController _controller)
      (CallFunction|HandleControllerConnectedInfo _controller))
    (:OnDisconnected
      (Demo|Controllers|HandleControllerDisconnected _controller))))

(fn ConstructionScript)

(fn HandleControllerConnectedInfo
  (params (ControllerInfo :type JSL4U%20Controller%20Info%20Structure))
  (bind (_bisjoyshockcontroller _deviceid _connectionid) (Utilities|Struct|BreakJSL4UControllerInfo ControllerInfo))
  (Utilities|FlowControl|Sequence
    (:then_0
      (bind (_playercontroller _localplayerindex) (Class|JoyShockSubsystem|EnsureLocalPlayerforController (Subsystems|GetJoyShockSubsystem) (.DeviceId (Utilities|Struct|BreakJSL4UControllerInfo ControllerInfo)) true)
        (:True
          (bind _has_mapping_context (CallFunction|EnsureDemoMappingContext _playercontroller))
          (if _has_mapping_context
            (Utilities|IsValid (Game|GetPlayerCharacter _localplayerindex)
              (:Is%20Not%20Valid
                (Class|GameModeBase|RestartPlayer (Game|GetGameMode) _playercontroller)))
            (else
              (Development|PrintString "Failed to configure mapping context"))))))
    (:then_1
      (if (not (.ReturnValue (Utilities|Map|Find (Variables|Demo|ControllerMirrors|GetMirrors%20By%20Connection%20ID) _connectionid)))
        (bind _returnvalue (Game|SpawnActorfromClass "/JoyShockLibrary4Unreal/BP_JoyShockControllerMirror.BP_JoyShockControllerMirror_C" (Math|Transform|MakeTransform (+ (Variables|Demo|ControllerMirrors|GetController%20Spawn%20Location) (* "0,250,0" (Utilities|Map|Length (Variables|Demo|ControllerMirrors|GetMirrors%20By%20Connection%20ID))))) "Undefined" "MultiplyWithRoot" 0 ControllerInfo 0))
        (Utilities|Map|Add (Variables|Demo|ControllerMirrors|GetMirrors%20By%20Connection%20ID) _connectionid _returnvalue)
        (Utilities|Map|Add (Variables|Demo|ControllerMirrors|GetMirrors%20By%20Device%20ID) _deviceid _returnvalue)
        (Demo|Diagnostics|RefreshDiagnosticsHUD)))))

(fn EnsureDemoMappingContext
  (params (Player%20Controller :type Player%20Controller%20Object%20Reference))
  (bind _returnvalue (PlayerController|LocalPlayerSubsystems|GetEnhancedInputLocalPlayerSubsystem Player%20Controller))
  (Utilities|IsValid _returnvalue
    (:Is%20Valid
      (if (.ReturnValue (Class|EnhancedInputSubsystemInterface|HasMappingContext _returnvalue "/JoyShockLibrary4Unreal/EnhancedInput/JoyShockInputMappingContext.JoyShockInputMappingContext"))
        (LocalVariables|SetHas%20Mapping%20Context? true)
        (else
          (Input|AddMappingContext _returnvalue "/JoyShockLibrary4Unreal/EnhancedInput/JoyShockInputMappingContext.JoyShockInputMappingContext" 0 "(bIgnoreAllPressedKeysUntilRelease=True,bForceImmediately=False,bNotifyUserSettings=False)")
          (LocalVariables|SetHas%20Mapping%20Context? true))))
    (:Is%20Not%20Valid
      (Development|PrintString "Enhanced Input subsystem invalid")
      (LocalVariables|SetHas%20Mapping%20Context? false)))
  (return (LocalVariables|GetHas%20Mapping%20Context?)))

(fn EnsureCharacterforController
  (params (Controller%20Info :type JSL4U%20Controller%20Info%20Structure))
  (bind (_playercontroller _localplayerindex) (Class|JoyShockSubsystem|EnsureLocalPlayerforController (Subsystems|GetJoyShockSubsystem) (.DeviceId (Utilities|Struct|BreakJSL4UControllerInfo Controller%20Info)) true)
    (:True
      (CallFunction|EnsureDemoMappingContext _playercontroller)
      (Utilities|IsValid (Pawn|GetControlledPawn _playercontroller)
        (:Is%20Not%20Valid
          (bind _outactors (Actor|GetAllActorsOfClass "/Script/Engine.PlayerStart"))
          (bind _returnvalue (Game|SpawnActorfromClass "/JoyShockLibrary4Unreal/BP_JoyShockCharacter.BP_JoyShockCharacter_C" (Transformation|GetActorTransform (Utilities|Array|Get(acopy) _outactors (Math|Integer|%(Integer) _localplayerindex (Utilities|Array|Length _outactors)))) "AdjustIfPossibleButAlwaysSpawn" "MultiplyWithRoot" 0 0))
          (Pawn|Possess _playercontroller _returnvalue)
          (return))))))

(fn HandleControllerDisconnected
  (params (JSL4UControllerInfo :type JSL4U%20Controller%20Info%20Structure%20%28by%20ref%29))
  (bind (_bisjoyshockcontroller _deviceid _connectionid) (Utilities|Struct|BreakJSL4UControllerInfo JSL4UControllerInfo))
  (bind _mirrors_by_connection_id (Variables|Demo|ControllerMirrors|GetMirrors%20By%20Connection%20ID))
  (bind (_value _returnvalue) (Utilities|Map|Find _mirrors_by_connection_id _connectionid))
  (if _returnvalue
    (Actor|DestroyActor _value)
    (Utilities|Map|Remove (Variables|Demo|ControllerMirrors|GetMirrors%20By%20Connection%20ID) _connectionid)
    (Utilities|Map|Remove (Variables|Demo|ControllerMirrors|GetMirrors%20By%20Device%20ID) _deviceid)))

(fn RefreshDiagnosticsHUD
  (if (Utilities|IsValid (Variables|Demo|Diagnostics|GetDiagnostics%20HUD))
    (Widget|RemovefromParent (Variables|Demo|Diagnostics|GetDiagnostics%20HUD)))
  (bind _returnvalue (UserInterface|CreateWidget "/JoyShockLibrary4Unreal/UI/WBP_JoyShockHUD.WBP_JoyShockHUD_C" (Game|GetPlayerController 0)))
  (Variables|Demo|Diagnostics|SetDiagnostics%20HUD _returnvalue)
  (Variables|/JoyShockLibrary4Unreal/UI/WBP_JoyShockHUD.WBP_JoyShockHUD_C|SetMirrors%20by%20Device%20ID _returnvalue (Variables|Demo|ControllerMirrors|GetMirrors%20By%20Device%20ID))
  (UserInterface|Viewport|AddtoViewport _returnvalue 0))