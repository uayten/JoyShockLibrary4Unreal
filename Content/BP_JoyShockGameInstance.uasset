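; BP_JoyShockGameInstance is a Game Instance that reports JoyShock controller connections and disconnections.
; On Init it prints a startup message and binds handlers to the JoyShock subsystem's connected and disconnected delegates.
; Each handler prints the device ID to screen, with the connect message held for a long duration and the disconnect's timeout flag unused.
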(event Custom|OnControllerConnected_Event
  (params (DeviceId :type Integer))
  (Development|PrintString (Utilities|String|Append "Controller Connected: " (Utilities|String|ToString(Integer) DeviceId)) true true "(R=0.000000,G=0.660000,B=1.000000,A=1.000000)" 1e+02))

(event Custom|OnControllerDisconnected_Event
  (params (DeviceId :type Integer) (bTimedOut :type Boolean))
  (Development|PrintString (Utilities|String|Append "Controller Disconnected: " (Utilities|String|ToString(Integer) DeviceId))))

(event EventInit
  (Development|PrintString "Game Instance Initialized")
  (EventDispatchers|AssignOnControllerConnected (Subsystems|GetJoyShockSubsystem) (delegate Custom|OnControllerConnected_Event))
  (EventDispatchers|AssignOnControllerDisconnected (Subsystems|GetJoyShockSubsystem) (delegate Custom|OnControllerDisconnected_Event)))