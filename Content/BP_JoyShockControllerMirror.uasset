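; Actor that mirrors one physical controller in the world through JSL4U, showing a matching mesh and following its motion.
; Joy-Cons refresh on pairing changes, with body colors, player LEDs and a grip mesh when joined; Pro Controllers use a DualSense placeholder.
; Tick copies orientation in rotation mode, or maps yaw/pitch offset from the BeginPlay pose to clamped movement in aim mode.
; Events forward gyro space and calibration commands to the device.
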(event Custom|On/Off%20Rotation%20Mode
  (params (bRotationMode :type Boolean))
  (Variables|Default|SetRotation%20Mode? bRotationMode))

(event Custom|On/Off%20Aim%20Mode
  (params (bAimMode :type Boolean))
  (bind _output_get (Variables|Default|SetAim%20Mode? bAimMode))
  (if (not _output_get)
    (Transformation|SetActorLocation (Variables|Default|GetHome%20Location) false false)))

(event Custom|Set%20Gyro%20Calibration%20Mode
  (params (Mode :type EJSL4UGyroCalibrationMode%20Enum :default "Automatic"))
  (Class|JoyShockLibrary|JSL4USetGyroCalibrationMode (Variables|Default|GetDeviceID) Mode))

(event Custom|Start%20Manual%20Gyro%20Calibration
  (Class|JoyShockLibrary|JSL4UStartGyroCalibration (Variables|Default|GetDeviceID)))

(event Custom|Stop%20Manual%20Gyro%20Calibration
  (Class|JoyShockLibrary|JSL4UStopGyroCalibration (Variables|Default|GetDeviceID)))

(event Custom|Gyro%20Space:%20Local
  (Class|JoyShockLibrary|JSL4USetGyroSpace (Variables|Default|GetDeviceID) "LocalSpace"))

(event Custom|Gyro%20Space:%20Player
  (Class|JoyShockLibrary|JSL4USetGyroSpace (Variables|Default|GetDeviceID) "PlayerSpace"))

(event Custom|Gyro%20Space:%20World
  (Class|JoyShockLibrary|JSL4USetGyroSpace (Variables|Default|GetDeviceID) "WorldSpace"))

(event EventTick
  (params (DeltaSeconds :type Float%20%28single-precision%29))
  (bind _deviceid (Variables|Default|GetDeviceID))
  (bind _natural_rotation (Variables|Default|GetNatural%20Rotation))
  (bind _returnvalue (Class|JoyShockLibrary|JSL4UGetMotionState _deviceid))
  (bind _returnvalue_2 (Class|KismetMathLibrary|QuatRotator (.orientation _returnvalue)))
  (bind _returnvalue_3 (Math|Rotator|Delta(Rotator) _returnvalue_2 _natural_rotation))
  (bind (_roll _pitch _yaw) (Math|Rotator|BreakRotator _returnvalue_3))
  (Utilities|FlowControl|Sequence
    (:then_0
      (if (Variables|Default|GetRotation%20Mode?)
        (Transformation|SetRelativeRotation (Variables|Default|GetSM_Controller) (Class|KismetMathLibrary|QuatRotator (.orientation (Class|JoyShockLibrary|JSL4UGetMotionState (Variables|Default|GetDeviceID)))) false false)))
    (:then_1
      (if (Variables|Default|GetAim%20Mode?)
        (Transformation|SetRelativeLocation (Variables|Default|GetSM_Controller) (+ (Math|Vector|MakeVector 0.0 (* (Math|Float|Clamp(Float) (/ _yaw (Variables|Default|GetMax%20Angle)) -1.0) (Variables|Default|GetMove%20Range)) (* (Math|Float|Clamp(Float) (/ _pitch (Variables|Default|GetMax%20Angle)) -1.0) (Variables|Default|GetMove%20Range))) (Variables|Default|GetHome%20Location)) false false)))))

(event EventBeginPlay
  (bind _controller (Variables|Controller|GetController))
  (bind _controllertype (Utilities|Struct|BreakJSL4UControllerInfo _controller))
  (bind _output_get (Variables|Default|SetDeviceID (.DeviceId (Utilities|Struct|BreakJSL4UControllerInfo (Variables|Controller|GetController)))))
  (Variables|Default|SetNatural%20Rotation (Class|KismetMathLibrary|QuatRotator (.orientation (Class|JoyShockLibrary|JSL4UGetMotionState _output_get))))
  (Variables|Default|SetHome%20Location (Transformation|GetActorLocation))
  (if (or (Utilities|Enum|Equal(Enum) _controllertype "JoyConLeft") (Utilities|Enum|Equal(Enum) _controllertype "JoyConRight"))
    (|WaitforJoyConPairingChanges
      (:then
        (CallFunction|ApplyControllerAppearance(Joycons)))
      (:OnJoined
        (CallFunction|ApplyControllerAppearance(Joycons) :!label _label))
      (:OnSeparated
        (goto _label)))
    (else
      (CallFunction|ApplyControllerAppearance(ExceptJoycons)))))

(fn ConstructionScript)

(fn ApplyControllerAppearance(ExceptJoycons)
  (switch Utilities|FlowControl|Switch|SwitchonEJSL4UControllerType (.controllertype (Variables|Controller|GetController))
    (:Undefined
      (Components|StaticMesh|SetStaticMesh (Variables|Default|GetSM_Controller) "/JoyShockLibrary4Unreal/Meshes/Sony/DualSense/SM_Dual_Sense.SM_Dual_Sense" :!label _label))
    (:ProController
      ;[0.15 0.15 0.15 0.5] Pro Controller meshes still missing
      (Components|StaticMesh|SetStaticMesh (Variables|Default|GetSM_Controller) "/JoyShockLibrary4Unreal/Meshes/Sony/DualSense/SM_Dual_Sense.SM_Dual_Sense" :!label _label_2))
    (:DualShock4
      (Components|StaticMesh|SetStaticMesh (Variables|Default|GetSM_Controller) "/JoyShockLibrary4Unreal/Meshes/Sony/DualShock4/Dual_Shock_4.Dual_Shock_4"))
    (:DualSense
      (goto _label))
    (:ProController2
      (goto _label_2))))

(fn SetNintendoPairingLed
  (Development|PrintString (Utilities|String|ToString(Integer) (Rendering|Material|GetMaterialIndex (Variables|Default|GetSM_Controller) "MI_PairingLed1"))))

(fn ApplyControllerAppearance(Joycons)
  (bind _deviceid (Variables|Default|GetDeviceID))
  (bind _deviceid_2 (Variables|Default|GetDeviceID))
  (bind (_primarycontroller _partnercontroller _returnvalue) (Class|JoyShockLibrary|JSL4UGetJoyConPair _deviceid))
  (Class|JoyShockLibrary|JSL4USetHomeLight _deviceid_2 0.0)
  (if (Class|JoyShockLibrary|JSL4UIsJoinPrimary _deviceid_2)
    (if _returnvalue
      ;[0.15 0.15 0.15 0.5] Merged Joycon
      (Variables|Controller|SetJoy-Con%20Primary _primarycontroller)
      (Variables|Controller|SetJoy-Con%20Partner _partnercontroller)
      (CallFunction|SetStaticMesh&ResetMaterials "/JoyShockLibrary4Unreal/Meshes/Nintendo/Joy-Con(Grip)/SM_Joy-Con_Grip.SM_Joy-Con_Grip")
      (Utilities|SetJoy-ConSingleColor (Variables|Controller|GetJoy-Con%20Primary))
      (Utilities|SetJoy-ConSingleColor (Variables|Controller|GetJoy-Con%20Partner))
      (Utilities|SetJoyconPairingLed)
      (else
        (switch Utilities|FlowControl|Switch|SwitchonEJSL4UControllerType (.ControllerType (Utilities|Struct|BreakJSL4UControllerInfo (Variables|Controller|GetController)))
          (:JoyConLeft
            (CallFunction|SetStaticMesh&ResetMaterials "/JoyShockLibrary4Unreal/Meshes/Nintendo/Joy-Con(L)/SM_Joy-Con_L.SM_Joy-Con_L"))
          (:JoyConRight
            (CallFunction|SetStaticMesh&ResetMaterials "/JoyShockLibrary4Unreal/Meshes/Nintendo/Joy-Con(R)/SM_Joy-Con_R.SM_Joy-Con_R")))
        ;[0.15 0.15 0.15 0.5] Sandalone Joycon
        (Utilities|SetJoy-ConSingleColor (Variables|Controller|GetController))
        (Utilities|SetJoyconPairingLed)))
    (else
      ;[0.15 0.15 0.15 0.5] Paired with another joy-con
      (Components|StaticMesh|SetStaticMesh (Variables|Default|GetSM_Controller) 0))))

(fn SetStaticMesh&ResetMaterials
  (params (NewMesh :type Static%20Mesh%20Object%20Reference))
  (Components|StaticMesh|SetStaticMesh (Variables|Default|GetSM_Controller) NewMesh)
  (for _index (range 0 (Rendering|Material|GetNumMaterials (Variables|Default|GetSM_Controller)))
    (Rendering|Material|SetMaterial (Variables|Default|GetSM_Controller) _index 0)))